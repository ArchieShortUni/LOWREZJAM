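; Player pixel character that uses directional flipbook animation and is viewed through the level's camera.
; On BeginPlay it switches the first player controller's view target to the Level_Camera actor.
; MovementChange compares CurrentMovementVector against eight directions to pick a movement flipbook while moving, with no idle case.
; Any damage destroys the actor outright, and its Destroyed event calls CharacterDeath.
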(event EventBeginPlay
  (Development|PrintString "new player spawned")
  (bind _returnvalue (Actor|GetActorOfClass "/Game/GameLogic/Level_Camera.Level_Camera_C"))
  (Game|Player|SetViewTargetwithBlend (Game|GetPlayerController 0) _returnvalue 0.0 "VTBlend_Linear" 0.0 false))

(event Collision|EventActorBeginOverlap
  (params (OtherActor :type Actor%20Object%20Reference)))

(event EventDestroyed
  (Default|CallCharacterDeath))

(event EventTakeDamage
  (Actor|DestroyActor))

(fn ConstructionScript)

(fn MovementChange
  (bind _currentmovementvector (Variables|Default|GetCurrentMovementVector))
  (if (Variables|Default|GetIsCharacterMoving)
    (if (Math|Vector|Equal(Vector) _currentmovementvector "-1.000000,0.000000, 0" 0.0001)
      (Sprite|SetFlipbook (Variables|Default|GetCharacterFlipbook) "/Game/Character/Flipbooks/Move_Up.Move_Up")
      (elif (Math|Vector|Equal(Vector) _currentmovementvector "1.000000,0.000000, 0" 0.0001)
        (Sprite|SetFlipbook (Variables|Default|GetCharacterFlipbook) "/Game/Character/Flipbooks/Move_Down.Move_Down")
        (elif (Math|Vector|Equal(Vector) _currentmovementvector "0.000000,-1.000000, 0" 0.0001)
          (Sprite|SetFlipbook (Variables|Default|GetCharacterFlipbook) "/Game/Character/Flipbooks/Move_Right.Move_Right")
          (elif (Math|Vector|Equal(Vector) _currentmovementvector "0.000000,1.000000, 0" 0.0001)
            (Sprite|SetFlipbook (Variables|Default|GetCharacterFlipbook) "/Game/Character/Flipbooks/Move_Left.Move_Left")
            (elif (Math|Vector|Equal(Vector) _currentmovementvector "1.000000,1.000000, 0" 0.0001)
              (Sprite|SetFlipbook (Variables|Default|GetCharacterFlipbook) "/Game/Character/Flipbooks/Move_Down_Left.Move_Down_Left")
              (elif (Math|Vector|Equal(Vector) _currentmovementvector "1.000000,-1.000000, 0" 0.0001)
                (Sprite|SetFlipbook (Variables|Default|GetCharacterFlipbook) "/Game/Character/Flipbooks/Move_Down_Right.Move_Down_Right")
                (elif (Math|Vector|Equal(Vector) _currentmovementvector "-1.000000,1.000000, 0" 0.0001)
                  (Sprite|SetFlipbook (Variables|Default|GetCharacterFlipbook) "/Game/Character/Flipbooks/Move_Up_Left.Move_Up_Left")
                  (elif (Math|Vector|Equal(Vector) _currentmovementvector "-1.000000,-1.000000, 0" 0.0001)
                    (Sprite|SetFlipbook (Variables|Default|GetCharacterFlipbook) "/Game/Character/Flipbooks/Move_Up_Right.Move_Up_Right")))))))))))